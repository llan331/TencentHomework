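; Grenade actor that explodes on a three-second fuse and destroys nearby targets.
; When the BeginPlay timer fires, it spawns an Explosion at its transform, copies that actor's RadialForce radius, then destroys itself.
; The Destroyed event uses the copied radius in a sphere overlap for WorldStatic BP_Target actors and destroys each one found.
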(event Custom|Detonate
  (bind _returnvalue (Game|SpawnActorfromClass "/Game/Blueprints/Actors/Explosion.Explosion_C" (Transformation|GetActorTransform) "Undefined" 0 0))
  (Variables|Default|SetRadius (Variables|/Script/Engine.RadialForceComponent|GetRadius (Variables|/Game/Blueprints/Actors/Explosion.Explosion_C|GetRadialForce _returnvalue)))
  (Actor|DestroyActor))

(event EventBeginPlay
  (Utilities|Time|SetTimerbyEvent (delegate Custom|Detonate) 3.0))

(event EventDestroyed
  (bind (_outactors _returnvalue) (Collision|SphereOverlapActors (Transformation|GetActorLocation) (Variables|Default|GetRadius) (Utilities|Array|MakeArray "ObjectTypeQuery1") "/Game/Blueprints/Actors/BP_Target.BP_Target_C"))
  (if _returnvalue
    (for _array_element _outactors
      (Actor|DestroyActor _array_element))))

(fn ConstructionScript)