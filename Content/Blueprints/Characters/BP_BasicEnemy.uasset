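; BP_BasicEnemy is an armed third-person character that keeps player-style input for movement, aiming, weapon toggling, shooting and grenade throwing, alongside enemy AI death handling.
; Server and Multicast events relay aim, equip state, montages, sounds and effects, while Tick updates animation values and camera zoom.
; PullTrigger takes any origin and direction for its line trace, which destroys targets or pushes static meshes.
; Depleted Health stops the AI controller's logic and plays a death montage before destruction.
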(event Custom|FireTrace
  (params (TraceOrigin :type Vector) (TraceDIrection :type Vector))
  ;[1 1 1] Fire
  (CallFunction|ServerGunFire (Variables|Default|GetHandGun) "/Game/Resources/Effects/MuzzleFlash/P_MF_Handgun.P_MF_Handgun" "Muzzle")
  (bind (_outhit _returnvalue) (Collision|LineTraceByChannel TraceOrigin (+ TraceOrigin (* TraceDIrection 1e+04)) "TraceTypeQuery1" false 0 "None"))
  (if _returnvalue
    (CallFunction|ServerPlayFire (.location _outhit) "/Game/Resources/Effects/Impacts/P_Imp_Default.P_Imp_Default")
    (bind _asbp_target (Utilities|Casting|CastToBP_Target (.hitactor _outhit))
      (:then
        (Actor|DestroyActor _asbp_target)
        (bind _asbp_player_controller (Utilities|Casting|CastToBP_PlayerController (Pawn|GetController)))
        (Default|IncreaseRecord (Variables|/Game/Blueprints/Characters/BP_PlayerController.BP_PlayerController_C|GetPlayerHUD _asbp_player_controller)))
      (:CastFailed
        (bind _asstatic_mesh_actor (Utilities|Casting|CastToStaticMeshActor (.hitactor _outhit)))
        (CallFunction|ServerAddImpulse (* (Math|Vector|Normalize (- (.traceend _outhit) (.tracestart _outhit))) 1e+05) (Variables|/Script/Engine.StaticMeshActor|GetStaticMeshComponent _asstatic_mesh_actor))))))

(event Custom|ServerSetIsArmed
  (params (Value :type Boolean))
  ;[1 1 1] Server
  (Variables|Default|SetIsArmed Value))

(event Custom|MulticastAttachWeapon
  (params (IsAttached :type Boolean))
  ;[1 1 1] Server
  (if IsAttached
    (Transformation|AttachComponentToComponent (Variables|Default|GetHandGun) (Variables|Character|GetMesh) "Socket_Handgun" "KeepRelative" "KeepRelative" "KeepRelative" true)
    (else
      (Transformation|AttachComponentToComponent (Variables|Default|GetHandGun) (Variables|Character|GetMesh) "Socket_Holster" "KeepRelative" "KeepRelative" "KeepRelative" true))))

(event Custom|ServerAddImpulse
  (params (vector :type Vector) (Component :type Primitive%20Component%20Object%20Reference))
  ;[1 1 1] Server
  (Physics|AddImpulse Component vector "None" false))

(event Custom|ServerSetAimPitch
  (params (AimPitch :type Float%20%28single-precision%29))
  (Variables|Default|SetAimPitch AimPitch))

(event Custom|ServerEnableAim
  (params (Enabled :type Boolean))
  (bind _charactermovement (Variables|Character|GetCharacterMovement))
  (bind _charactermovement_2 (Variables|Character|GetCharacterMovement))
  (if Enabled
    (Variables|/Script/Engine.CharacterMovementComponent|SetbOrientRotationToMovement _charactermovement false)
    (Variables|/Script/Engine.CharacterMovementComponent|SetMaxWalkSpeed _charactermovement_2 2e+02)
    (Variables|Default|SetbUseControllerRotationYaw true)
    (else
      (Variables|/Script/Engine.CharacterMovementComponent|SetbOrientRotationToMovement _charactermovement true)
      (Variables|/Script/Engine.CharacterMovementComponent|SetMaxWalkSpeed _charactermovement_2 6e+02)
      (Variables|Default|SetbUseControllerRotationYaw false))))

(event Custom|ServerSetGunLight
  (params (IsVisibility :type Boolean))
  ;[1 1 1] Server
  (CallFunction|MulticastGunLight IsVisibility))

(event Custom|MulticastGunLight
  (params (IsVisibility :type Boolean))
  ;[1 1 1] Server
  (Rendering|SetVisibility (Variables|Default|GetSpotLight) IsVisibility false))

(event Custom|ServerGunFire
  (params (component :type Scene%20Component%20Object%20Reference) (name :type Particle%20System%20Object%20Reference) (attachName :type Name))
  ;[1 1 1] Server
  (CallFunction|MulticastGunFire component name attachName))

(event Custom|MulticastGunFire
  (params (component :type Scene%20Component%20Object%20Reference) (name :type Particle%20System%20Object%20Reference) (attachName :type Name))
  ;[1 1 1] Server
  (Effects|SpawnEmitterAttached name component attachName))

(event Custom|ServerSetIsAiming
  (params (Value :type Boolean))
  ;[1 1 1] Server
  (Variables|Default|SetIsAiming Value))

(event Custom|ServerPlayFire
  (params (location :type Vector) (name :type Particle%20System%20Object%20Reference))
  ;[1 1 1] Server
  (CallFunction|MulticastPlayFire location name))

(event Custom|MulticastPlayFire
  (params (location :type Vector) (name :type Particle%20System%20Object%20Reference))
  ;[1 1 1] Server
  (Effects|SpawnEmitteratLocation name location))

(event Custom|ServerDecreaseHealth
  (params (Damage :type Float%20%28single-precision%29))
  (bind _output_get (Variables|Default|SetHealth (- (Variables|Default|GetHealth) Damage)))
  (if (<= _output_get 0.0)
    (CallFunction|Die)))

(event Custom|die
  (if (not (Variables|Default|GetIsDead))
    (Variables|Default|SetIsDead true)
    (bind _asbp_basic_enemy_controller (Utilities|Casting|CastToBP_BasicEnemyController (Pawn|GetController))
      (:then
        (AI|Logic|StopLogic (Variables|/Script/AIModule.AIController|GetBrainComponent _asbp_basic_enemy_controller) ""))
      (:CastFailed
        _))
    (Animation|Montage|PlayMontage (Variables|Character|GetMesh) "/Game/Animation/Death_Montage.Death_Montage" 1.5
      (:OnCompleted
        (Actor|DestroyActor)))))

(event Custom|PlaySound
  (params (Sound :type Sound%20Base%20Object%20Reference) (Location :type Vector))
  (CallFunction|MulticastPlaySound Location Sound))

(event Custom|MulticastPlaySound
  (params (NewParam :type Vector) (NewParam2 :type Sound%20Base%20Object%20Reference))
  (Audio|PlaySoundatLocation NewParam2 NewParam "0, 0, 0" 1.0 1.0 0.0 0 0 0))

(event Custom|PullTrigger
  (params (TraceOrigin :type Vector) (TraceDirection :type Vector))
  ;[1 1 1] Fire Action
  (CallFunction|ServerPlayMontage "/Game/Animation/HandGun/Shoot/Stand/ShootAdditive_Montage.ShootAdditive_Montage")
  (CallFunction|PlaySound "/Game/Resources/Sounds/Wav/Handgun/S_Handgun_Shoot.S_Handgun_Shoot" (Transformation|GetWorldLocation (Variables|Default|GetHandGun)))
  (CallFunction|FireTrace TraceOrigin TraceDirection))

(event Custom|ServerSetHasWeapon
  (params (Value :type Boolean))
  ;[1 1 1] Server
  (Variables|Default|SetHasWeapon Value))

(event Custom|ServerSetInAir
  (params (Value :type Boolean))
  ;[1 1 1] Server
  (Variables|Default|SetInAir Value))

(event Custom|ServerSetIsEquiping
  (params (Value :type Boolean))
  ;[1 1 1] Server
  (Variables|Default|SetIsEquiping Value))

(event Custom|ServerPlayMontage
  (params (Montage :type Anim%20Montage%20Object%20Reference))
  ;[1 1 1] Server
  (CallFunction|MulticastPlay Montage))

(event Custom|MulticastPlay
  (params (Montage :type Anim%20Montage%20Object%20Reference))
  ;[1 1 1] Server
  (Animation|Montage|MontagePlay (Components|SkeletalMesh|GetAnimInstance (Variables|Character|GetMesh)) Montage 1.0 "MontageLength" 0.0 true))

(event Custom|ServerAttachWeapon
  (params (IsAttached :type Boolean))
  ;[1 1 1] Server
  (CallFunction|MulticastAttachWeapon IsAttached))

(event EventTick
  (params (DeltaSeconds :type Float%20%28single-precision%29))
  (bind _returnvalue (Pawn|GetControlRotation :!class /Script/Engine.Pawn))
  (bind _charactermovement (Variables|Character|GetCharacterMovement))
  (bind _springarm (Variables|Default|GetSpringArm))
  (bind _returnvalue_2 (Pawn|Components|CharacterMovement|GetLastUpdateVelocity _charactermovement))
  (bind _returnvalue_3 (Math|Vector|VectorLength _returnvalue_2))
  ;[1 1 1] Tick Events
  (Variables|Default|SetSpeed _returnvalue_3)
  (Variables|Default|SetDirection (Math|Float|SelectFloat (.yaw (Math|Rotator|Delta(Rotator) _returnvalue (Math|Rotator|MakeRotfromX (Transformation|GetVelocity)))) 0.0 (>= _returnvalue_3 5e+01)))
  (CallFunction|ServerSetAimPitch (Math|Float|Clamp(Float) (.pitch (Math|Rotator|Delta(Rotator) _returnvalue (Transformation|GetActorRotation))) -85.0 85.0))
  (Variables|/Script/Engine.SpringArmComponent|SetTargetArmLength _springarm (Math|Float|Lerp (Variables|/Script/Engine.SpringArmComponent|GetTargetArmLength _springarm) (Variables|Default|GetTargetSpringArmLength) (* (Utilities|Time|GetWorldDeltaSeconds) 1e+01))))

(event Input|ActionEvents|InputActionAim
  (params (Key :type Key%20Structure :default "None"))
  (bind _charactermovement (Variables|Character|GetCharacterMovement))
  (bind _charactermovement_2 (Variables|Character|GetCharacterMovement))
  (bind _isarmed (Variables|Default|GetIsArmed))
  ;[1 1 1] Aim Action
  (:Pressed
    (if (not (AI|Components|NavMovement|IsFalling (Variables|Character|GetCharacterMovement)))
      (if _isarmed
        (CallFunction|ServerSetIsAiming true)
        (CallFunction|ServerEnableAim true)
        (Variables|/Script/Engine.CharacterMovementComponent|SetbOrientRotationToMovement _charactermovement_2 false)
        (Variables|/Script/Engine.CharacterMovementComponent|SetMaxWalkSpeed _charactermovement 2e+02)
        (Variables|Default|SetbUseControllerRotationYaw true)
        (Variables|Default|SetTargetSpringArmLength 1e+02)
        (Variables|Default|SetSensityNormal 0.25)
        (CallFunction|ServerSetGunLight true))))
  (:Released
    (if _isarmed
      (CallFunction|ServerSetIsAiming false)
      (CallFunction|ServerEnableAim false)
      (Variables|/Script/Engine.CharacterMovementComponent|SetbOrientRotationToMovement _charactermovement_2 true)
      (Variables|/Script/Engine.CharacterMovementComponent|SetMaxWalkSpeed _charactermovement 6e+02)
      (Variables|Default|SetbUseControllerRotationYaw false)
      (Variables|Default|SetTargetSpringArmLength 2e+02)
      (Variables|Default|SetSensityNormal 0.5)
      (CallFunction|ServerSetGunLight false))))

(event Input|ActionEvents|InputActionToggleWeapon
  (params (Key :type Key%20Structure :default "None"))
  ;[1 1 1] ToggleWeapon Action
  (:Pressed
    (if (and (Variables|Default|GetHasWeapon) (not (Variables|Default|GetIsAiming)))
      (if (Variables|Default|GetIsArmed)
        (CallFunction|ServerPlayMontage "/Game/Animation/HandGun/Action/A_HG_Unequip_Montage.A_HG_Unequip_Montage")
        (CallFunction|ServerSetIsEquiping true)
        (Utilities|FlowControl|Delay 0.5)
        (CallFunction|ServerAttachWeapon false)
        (CallFunction|ServerSetIsArmed false)
        (CallFunction|ServerSetIsEquiping false)
        (else
          (CallFunction|ServerPlayMontage "/Game/Animation/HandGun/Action/A_HG_Equip_Montage.A_HG_Equip_Montage")
          (CallFunction|ServerSetIsEquiping true)
          (Utilities|FlowControl|Delay 0.2)
          (CallFunction|ServerAttachWeapon true)
          (CallFunction|ServerSetIsArmed true)
          (CallFunction|ServerSetIsEquiping false))))))

(event Input|ActionEvents|InputActionJump
  (params (Key :type Key%20Structure :default "None"))
  ;[1 1 1] Input
  (:Pressed
    (Character|Jump)))

(event Input|ActionEvents|InputActionGrenades
  (params (Key :type Key%20Structure :default "None"))
  (bind _camera (Variables|Default|GetCamera))
  (bind _returnvalue (Transformation|GetWorldRotation _camera))
  ;[1 1 1] Input
  (:Pressed
    (bind _returnvalue_2 (Game|SpawnActorfromClass "/Game/Blueprints/Actors/Grenade.Grenade_C" (Math|Transform|MakeTransform (+ (Transformation|GetActorLocation) (* (Math|Vector|GetForwardVector (Variables|Default|GetCamera)) 1e+01)) _returnvalue "1,1,1") "Undefined" 0 0))
    (Physics|SetPhysicsLinearVelocity (Variables|/Game/Blueprints/Actors/Grenade.Grenade_C|GetSM_M_67 _returnvalue_2) (* (+ (Math|Vector|GetForwardVector _returnvalue) "0,0.000000,0.800000") 1e+03) false "None")))

(event Input|AxisEvents|InputAxisRight
  (params (AxisValue :type Float%20%28single-precision%29))
  ;[1 1 1] Input
  (Pawn|Input|AddMovementInput (Math|Vector|GetRightVector (Pawn|GetControlRotation :!class /Script/Engine.Pawn)) AxisValue false))

(event Input|AxisEvents|InputAxisTurn
  (params (AxisValue :type Float%20%28single-precision%29))
  ;[1 1 1] Input
  (Pawn|Input|AddControllerYawInput (* AxisValue (Variables|Default|GetSensityNormal))))

(event Input|AxisEvents|InputAxisLookUp
  (params (AxisValue :type Float%20%28single-precision%29))
  ;[1 1 1] Input
  (Pawn|Input|AddControllerPitchInput (* (* AxisValue -1.0) (Variables|Default|GetSensityNormal))))

(event Input|AxisEvents|InputAxisForward
  (params (AxisValue :type Float%20%28single-precision%29))
  ;[1 1 1] Input
  (Pawn|Input|AddMovementInput (Math|Vector|GetForwardVector (Pawn|GetControlRotation :!class /Script/Engine.Pawn)) AxisValue false))

(event Input|MouseEvents|LeftMouseButton
  (params (Key :type Key%20Structure :default "None"))
  (bind _camera (Variables|Default|GetCamera))
  ;[1 1 1] Fire Action
  (:Pressed
    (if (and (Variables|Default|GetIsAiming) (not (Variables|Default|GetIsEquiping)))
      (CallFunction|PullTrigger (Transformation|GetWorldLocation _camera) (Math|Vector|GetForwardVector (Transformation|GetWorldRotation _camera))))))

(fn ConstructionScript)

(fn OnRepHealth
  (if (<= (Variables|Default|GetHealth) 0.0)
    (CallFunction|Die)))