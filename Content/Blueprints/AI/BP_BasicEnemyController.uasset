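; AI controller for the basic enemy that runs its behavior tree and tracks the player through perception.
; Perception updates store or clear the sensed player and the sight flag, clearing the Player blackboard key when sight is lost.
; While the player is sensed and the enemy has health, Tick writes the player's location to that key and interpolates the pawn's rotation to face the player.
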(event OnTargetPerceptionUpdated(AIPerception)
  (params (Actor :type Actor%20Object%20Reference) (Stimulus :type AI%20Stimulus%20Structure))
  (Utilities|Casting|CastToBP_Player Actor)
  (if (.bSuccessfullySensed (Utilities|Struct|BreakAIStimulus Stimulus))
    (Variables|Default|SetHasPlayerSight? true)
    (Variables|Default|SetPlayer Actor)
    (else
      (AI|Components|Blackboard|ClearValue (Variables|Default|GetBlackboard) (Utilities|Name|MakeLiteralName "Player"))
      (Variables|Default|SetHasPlayerSight? false)
      (Variables|Default|SetPlayer 0))))

(event EventBeginPlay
  (AI|RunBehaviorTree "/Game/Blueprints/AI/BT_BasicEnemy.BT_BasicEnemy"))

(event EventPossess
  (params (PossessedPawn :type Pawn%20Object%20Reference)))

(event EventTick
  (params (DeltaSeconds :type Float%20%28single-precision%29))
  (bind _returnvalue (Pawn|GetControlledPawn))
  (if (and (Variables|Default|GetHasPlayerSight?) (> (Variables|/Game/Blueprints/Characters/BP_BasicEnemy.BP_BasicEnemy_C|GetHealth (.AsBP%20Basic%20Enemy (Utilities|Casting|CastToBP_BasicEnemy (Pawn|GetControlledPawn)))) 0.0))
    (AI|Components|Blackboard|SetValueasVector (Variables|Default|GetBlackboard) (Utilities|Name|MakeLiteralName "Player") (Transformation|GetActorLocation (Variables|Default|GetPlayer)))
    (Transformation|SetActorRotation _returnvalue (Math|Interpolation|RInterpTo (Transformation|GetActorRotation _returnvalue) (Math|Rotator|MakeRotfromX (- (Transformation|GetActorLocation (Variables|Default|GetPlayer)) (Transformation|GetActorLocation _returnvalue))) (Utilities|Time|GetWorldDeltaSeconds) 0.0))))

(fn ConstructionScript)